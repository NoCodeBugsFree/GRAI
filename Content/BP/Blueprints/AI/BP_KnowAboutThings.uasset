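; Behavior tree node that tracks whether the AI currently sees anything other than BP_GoodFood.
; Each AI tick, it scans the controller's sight-perceived actors and stops at the first whose class is not exactly BP_GoodFood.
; It writes the result to the KnowAboutStuff blackboard bool, which is false when nothing or only BP_GoodFood is seen.
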(event `self.ReceiveTickAI`
  (params (OwnerController :type "AIController Object Reference") (ControlledPawn :type "Pawn Object Reference") (DeltaSeconds :type "Float (single-precision)"))
  (set `self.FoundItem` false)
  (for _array_element (`AIPerceptionComponent.GetPerceivedActors` (`AIController.GetAIPerceptionComponent` OwnerController) "/Script/AIModule.AISense_Sight")
    (if (!= (`GameplayStatics.GetObjectClass` _array_element) "/Game/BP/Blueprints/Pickups/BP_GoodFood.BP_GoodFood_C")
      (set `self.FoundItem` true)
      (break)))
  (`BTFunctionLibrary.SetBlackboardValueAsBool` (`self.KnowAboutStuff`) (`self.FoundItem`)))