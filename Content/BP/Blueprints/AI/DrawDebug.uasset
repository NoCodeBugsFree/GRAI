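; Behavior tree task that draws a debug arrow from the controlled pawn to its current target.
; On execute it points at the DesiredObject blackboard actor's location when that actor is valid, otherwise at the Destination blackboard vector.
; The orange arrow stays visible briefly, and the task always finishes successfully right away.
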(event `self.ReceiveExecuteAI`
  (params (OwnerController :type "AIController Object Reference") (ControlledPawn :type "Pawn Object Reference"))
  (bind _returnvalue (`Actor.K2_GetActorLocation` ControlledPawn))
  (bind _returnvalue_2 (`BTFunctionLibrary.GetBlackboardValueAsActor` (`self.DesiredObject`)))
  (`/Engine/EditorBlueprintResources/StandardMacros.IsValid` _returnvalue_2
    (:`Is Valid`
      (`KismetSystemLibrary.DrawDebugArrow` _returnvalue (`Actor.K2_GetActorLocation` _returnvalue_2) 10.0 (struct :`R` 1.0 :`G` 0.088419 :`A` 1.0) 2.0 5.0)
      (`self.FinishExecute` true))
    (:`Is Not Valid`
      (`KismetSystemLibrary.DrawDebugArrow` _returnvalue (`BTFunctionLibrary.GetBlackboardValueAsVector` (`self.Destination`)) 10.0 (struct :`R` 1.0 :`G` 0.088419 :`A` 1.0) 2.0 5.0)
      (`self.FinishExecute` true))))