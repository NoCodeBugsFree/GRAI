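; Behavior Tree task that switches the AI-controlled pawn between walk and run speed.
; It reads a boolean Blackboard key, optionally inverted, and sets the Character Movement Component's max walk speed to WalkSpeed when true or RunSpeed when false.
; The task finishes immediately, succeeding after the change or failing if the pawn's movement component is not a Character Movement Component.
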(event `self.ReceiveExecuteAI`
  (params (OwnerController :type "AIController Object Reference") (ControlledPawn :type "Pawn Object Reference"))
  (bind _returnvalue (`BTFunctionLibrary.GetBlackboardValueAsBool` (`self.MoveRateKey`)))
  (bind _ascharacter_movement_component (cast `CharacterMovementComponent` (`Pawn.GetMovementComponent` ControlledPawn))
    (:`then`
      (if (select `bool` (`self.bInvert`) :`false` _returnvalue :`true` (not _returnvalue))
        (set `CharacterMovementComponent.MaxWalkSpeed` (`self.WalkSpeed`) _ascharacter_movement_component)
        (else
          (set `CharacterMovementComponent.MaxWalkSpeed` (`self.RunSpeed`) _ascharacter_movement_component)))
      (`self.FinishExecute` true))
    (:`CastFailed`
      (`self.FinishExecute` false))))