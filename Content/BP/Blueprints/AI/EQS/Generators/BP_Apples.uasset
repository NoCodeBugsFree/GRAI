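; BP_Apples is an EQS generator that supplies food items an AI character can see and that match a desired stat.
; It identifies the querying pawn by searching all GRAI_AI_Charater actors for one located at the first context location, within a small tolerance.
; It then reads that pawn's sight-perceived actors and adds each BP_GoodFood within Range whose PrimaryStatIndex equals DesiredStat.
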(fn `DoItemGeneration`
  (params (ContextLocations :type "Array of Vector Structure (by ref)"))
  (locals (`Found AI Pawn` :type "GRAI_AI_Charater Object Reference"))
  (bind _output (`|GetArrayItem` ContextLocations))
  (bind _outactors (`GameplayStatics.GetAllActorsOfClass` "/Script/GRAI.GRAI_AI_Charater"))
  (for _array_element _outactors
    (if (== (`Actor.K2_GetActorLocation` _array_element) _output :`ErrorTolerance` 10.0)
      (set `local.Found AI Pawn` _array_element)
      (break)))
  (for _array_element_2 (`AIPerceptionComponent.GetPerceivedActors` (`AIController.GetAIPerceptionComponent` (`AIBlueprintHelperLibrary.GetAIController` (`local.Found AI Pawn`))) "/Script/AIModule.AISense_Sight")
    (bind _asbp_good_food (cast `/Game/BP/Blueprints/Pickups/BP_GoodFood` _array_element_2))
    (if (and (> (`self.Range`) (`KismetMathLibrary.VSize` (- (`Actor.K2_GetActorLocation` _array_element_2) _output))) (== (`BaseFood.PrimaryStatIndex` _asbp_good_food) (`self.DesiredStat`)))
      (`self.AddGeneratedActor` _asbp_good_food)))
  (return))