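; EQS generator that yields the trees an AI character's controller knows of whose primary stat index matches DesiredStat.
; It identifies the querying pawn indirectly, scanning all GRAI_AI_Charater actors for the first within 10 units of the first context location.
; It then filters the Trees list on that pawn's GRAI_AIC controller and adds matches as generated actors.
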(fn `DoItemGeneration`
  (params (ContextLocations :type "Array of Vector Structure (by ref)"))
  (locals (`Found AI Pawn` :type "GRAI_AI_Charater Object Reference"))
  (bind _outactors (`GameplayStatics.GetAllActorsOfClass` "/Script/GRAI.GRAI_AI_Charater"))
  (for _array_element _outactors
    (if (== (`Actor.K2_GetActorLocation` _array_element) (`|GetArrayItem` ContextLocations) :`ErrorTolerance` 10.0)
      (set `local.Found AI Pawn` _array_element)
      (break)))
  (for _array_element_2 (`GRAI_AIC.Trees` (cast `GRAI_AIC` (`AIBlueprintHelperLibrary.GetAIController` (`local.Found AI Pawn`)) :!pure true))
    (if (== (`Tree.PrimaryStatIndex` _array_element_2) (`self.DesiredStat`))
      (`self.AddGeneratedActor` null)))
  (return))