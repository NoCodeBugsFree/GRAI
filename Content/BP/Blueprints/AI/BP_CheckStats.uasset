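; Behavior tree tick logic that picks which of an AI character's stats most needs attention and writes it to the blackboard.
; Each tick it scores every entry in the cached BP_AICharacter's AIStats by percentage deficit times desirability, keeping the highest at or above StatLowLevel.
; It writes the chosen index and sets FindFoodKey.
; PossiblyFoundStat starts true each tick, so FindFoodKey is always set true, even when no stat qualifies.
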(event `self.ReceiveTickAI`
  (params (OwnerController :type "AIController Object Reference") (ControlledPawn :type "Pawn Object Reference") (DeltaSeconds :type "Float (single-precision)"))
  (set `self.PossiblyFoundStat` true)
  (`/Engine/EditorBlueprintResources/StandardMacros.IsValid` (`self.AIPawn`)
    (:`Is Valid`
      _)
    (:`Is Not Valid`
      (bind _asbp_aicharacter (cast `/Game/BP/Blueprints/AI/BP_AICharacter` ControlledPawn))
      (set `self.AIPawn` _asbp_aicharacter)))
  (set `self.TestValue` 0.0)
  (for (_array_element _array_index) (`GRAI_AI_Charater.AIStats` (`self.AIPawn`))
    (bind _returnvalue (* (* (- 1.0 (/ (- (`.CurrentStatValue` (break `AIStat` _array_element)) (`.StatMin` (break `AIStat` _array_element))) (- (`.StatMax` (break `AIStat` _array_element)) (`.StatMin` (break `AIStat` _array_element))))) 100.0) (`.StatDesirability` (break `AIStat` _array_element))))
    (if (>= _returnvalue (`self.StatLowLevel`))
      (set `self.PossiblyFoundStat` true)
      (if (> _returnvalue (`self.TestValue`))
        (set `self.ChosenStat` _array_index)
        (set `self.TestValue` _returnvalue))))
  (if (`self.PossiblyFoundStat`)
    (`BTFunctionLibrary.SetBlackboardValueAsInt` (`self.KeyDesiredStat`) (`self.ChosenStat`))
    (`BTFunctionLibrary.SetBlackboardValueAsBool` (`self.FindFoodKey`) true)
    (else
      (`BTFunctionLibrary.SetBlackboardValueAsBool` (`self.FindFoodKey`)))))