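; BP_GRAI_PC is a player controller that moves and rotates a possessed camera-style pawn.
; Movement axes offset the pawn horizontally relative to control rotation, without sweep, and align its ControllerArrow.
; Tick-fed gates, opened while mouse buttons are held, time presses against ClickThreshold to separate clicks from holds.
; A right hold turns control yaw and the SpringArm's pitch and yaw; click and left-hold actions are empty.
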(event `InputAxis|MoveForward`
  (params (AxisValue :type "Float (single-precision)"))
  (bind _returnvalue (`self.GetControlRotation`))
  ;[0 0.2837 1] Movement
  (`self.K2_AddActorLocalOffset` (`self.PossessedPawnBP`) (* (* (+ (* (`KismetMathLibrary.GetForwardVector` _returnvalue) AxisValue) (* (`KismetMathLibrary.GetRightVector` _returnvalue) (stale `InputAxis|MoveRight` AxisValue))) (`self.MovementRate`)) (1.0 1.0 0.0)) false false :!label _label)
  (`SceneComponent.K2_SetWorldRotation` (`/Game/BP/Blueprints/Core/BP_GRAI_PlayerPawn.ControllerArrow` (`self.PossessedPawnBP`)) (`self.GetControlRotation`) false false))

(event `InputAxis|MoveRight`
  (params (AxisValue :type "Float (single-precision)"))
  ;[0 0.2837 1] Movement
  (goto _label))

(event `Key|LeftMouseButton`
  (params (Key :type "Key Structure"))
  (bind _leftclickholdcounter (`self.LeftClickHoldCounter`))
  ;[0 0.2837 1] Mouse
  (:`Pressed`
    (`|ExecutionSequence`
      (:`then_0`
        (goto _label_2 :!via `Open`))))
  (:`Released`
    (if (not (`self.bLeftClick`))
      _
      (else
        _))
    (set `self.LeftClickHoldCounter` 0.0)
    (set `self.bLeftClick` true)
    (goto _label_2 :!via `Close`)))

(event `self.ReceiveTick`
  (params (DeltaSeconds :type "Float (single-precision)"))
  (bind _leftclickholdcounter (`self.LeftClickHoldCounter`))
  (bind _rightclickholdcounter (`self.RightClickHoldCounter`))
  (bind _springarm (`/Game/BP/Blueprints/Core/BP_GRAI_PlayerPawn.SpringArm` (`self.PossessedPawnBP`)))
  ;[0 0.2837 1] Mouse
  (set `self.DeltaSeconds` DeltaSeconds)
  (`|ExecutionSequence`
    (:`then_0`
      (`/Engine/EditorBlueprintResources/StandardMacros.Gate` true :!label _label_2
        (:`Exit`
          (if (`self.bLeftClick`)
            (if (>= _leftclickholdcounter (`self.ClickThreshold`))
              (set `self.bLeftClick` false)
              (else
                (set `self.LeftClickHoldCounter` (+ (`self.DeltaSeconds`) _leftclickholdcounter))))))))
    (:`then_1`
      (`/Engine/EditorBlueprintResources/StandardMacros.Gate` true :!label _label_3
        (:`Exit`
          (if (`self.bRightClick`)
            (if (>= _rightclickholdcounter (`self.ClickThreshold`))
              (set `self.bRightClick` false)
              (else
                (set `self.RightClickHoldCounter` (+ (`self.DeltaSeconds`) _rightclickholdcounter))))
            (else
              (`self.SetControlRotation` (`KismetMathLibrary.MakeRotator` 0.0 0.0 (+ (`self.GetInputAxisKeyValue`) (.yaw (`self.GetControlRotation`)))))
              (`SceneComponent.K2_SetWorldRotation` _springarm (`KismetMathLibrary.MakeRotator` 0.0 (+ (`self.GetInputAxisKeyValue`) (.pitch (`SceneComponent.K2_GetComponentRotation` _springarm))) (+ (`self.GetInputAxisKeyValue`) (.yaw (`SceneComponent.K2_GetComponentRotation` _springarm)))) false false))))))))

(event `Key|RightMouseButton`
  (params (Key :type "Key Structure"))
  ;[0 0.2837 1] Mouse
  (:`Pressed`
    (goto _label_3 :!via `Open`))
  (:`Released`
    (if (not (`self.bRightClick`))
      _
      (else
        _))
    (set `self.RightClickHoldCounter` 0.0)
    (set `self.bRightClick` true)
    (goto _label_3 :!via `Close`)))

(fn `UserConstructionScript`)